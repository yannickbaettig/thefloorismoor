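; Shared camera for two local players that keeps both framed by following their midpoint and zooming with their separation.
; BeginPlay caches players 0 and 1 and the spring arm's starting position.
; Each Tick measures player distance and midpoint, then eases arm length toward that distance within fixed limits.
; The spring arm's X and Z track the midpoint through FInterpTo, while Y stays locked for a side-on style view.
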(event `self.ReceiveBeginPlay`
  (`|ExecutionSequence`
    (:`then_0`
      (set `self.P1` (`GameplayStatics.GetPlayerCharacter` 0))
      (set `self.P2` (`GameplayStatics.GetPlayerCharacter` 1)))
    (:`then_1`
      (set `self.CameraXPosition` (.x (`SceneComponent.K2_GetComponentLocation` (`self.SpringArm`))))
      (set `self.CameraZPosition` (.z (`SceneComponent.K2_GetComponentLocation` (`self.SpringArm`))))
      (set `self.CameraYPosition` (.y (`SceneComponent.K2_GetComponentLocation` (`self.SpringArm`)))))))

(event `self.ReceiveTick`
  (params (DeltaSeconds :type "Float (single-precision)"))
  (set `self.Delta` DeltaSeconds)
  (`self.SetDistancseBetweenPlayers`)
  (`self.SetCenterPosition`)
  (`self.CameraZoom`)
  (`self.SetCameraPosition`))

(event `CameraZoom`
  (bind _springarm (`self.SpringArm`))
  ;[1 1 1] Camera Zoom
  (set `SpringArmComponent.TargetArmLength` (`KismetMathLibrary.FInterpTo` (`SpringArmComponent.TargetArmLength` _springarm) (`KismetMathLibrary.FClamp` (`self.DistanceBetweenPlayers`) 750.0 1500.0) (`self.Delta`) 1.0) _springarm))

(event `SetDistancseBetweenPlayers`
  ;[1 1 1] Distance Between Players
  (set `self.DistanceBetweenPlayers` (`self.GetDistanceTo` (`self.P1`) (`self.P2`))))

(event `SetCenterPosition`
  ;[1 1 1] Set Center Position Between Players
  (set `self.CenterPosition` (/ (+ (`self.K2_GetActorLocation` (`self.P1`)) (`self.K2_GetActorLocation` (`self.P2`))) (2.0 2.0 2.0))))

(event `SetCameraPosition`
  ;[1 1 1] Set Camera Position
  (set `self.CameraXPosition` (`KismetMathLibrary.FInterpTo` (`self.CameraXPosition`) (.x (`self.CenterPosition`)) (`self.Delta`)))
  (set `self.CameraZPosition` (`KismetMathLibrary.FInterpTo` (`self.CameraZPosition`) (.z (`self.CenterPosition`)) (`self.Delta`)))
  (`SceneComponent.K2_SetWorldLocation` (`self.SpringArm`) (`KismetMathLibrary.MakeVector` (`self.CameraXPosition`) (`self.CameraYPosition`) (`self.CameraZPosition`)) false false))

(fn `UserConstructionScript`)