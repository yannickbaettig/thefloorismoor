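; Paper2D side-scrolling player character with a replicated sprite that runs along X, jumps and flips its controller yaw to face the movement direction.
; A jump pressed at a jump count of one spins the sprite in quarter turns, paced by a custom delay-driven for-loop macro.
; Movement input refreshes the animation, using velocity and falling state to select an idle, run or jump flipbook.
; A rotation timeline is left unconnected.
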(event `self.ReceiveBeginPlay`
  (`ActorComponent.SetIsReplicated` (`self.Sprite`) true) ; replication
)

(event `InputAxis|MoveRight`
  (params (AxisValue :type "Float (single-precision)"))
  ;[1 1 1] Movement
  (`self.AddMovementInput` (1.0 0.0 0.0) AxisValue)
  (`self.UpdateAnimation`)
  (`/Engine/EditorBlueprintResources/StandardMacros.CompareFloat` AxisValue
    (:`>`
      (`Controller.SetControlRotation` (`self.GetController`) (`KismetMathLibrary.MakeRotator` 0.0 0.0 180.0)))
    (:`<`
      (`Controller.SetControlRotation` (`self.GetController`) (`KismetMathLibrary.MakeRotator` 0.0 0.0 0.0)))))

(event `InputAction|Jump`
  (params (Key :type "Key Structure"))
  ;[1 1 1] Jumping
  (:`Pressed`
    (if (== (`self.JumpCurrentCount`) 1)
      (`self.Jump`)
      (`self.ForLoopWithDelay` 1 4 :!label _label
        (:`Loop Body`
          (`SceneComponent.K2_AddLocalRotation` (`self.Sprite`) (struct :`Pitch` -90.0) false false))
        (:`DelayOut`
          (`KismetSystemLibrary.Delay` 0.1)
          (goto _label :!via `DelayIn`)))
      (else
        (`self.Jump`))))
  (:`Released`
    (`self.StopJumping`)))

(event `UpdateAnimation`
  ;[1 1 1] Animation
  (set `self.Is Moving` (> (`KismetMathLibrary.VSize` (`self.GetVelocity`)) 0.0))
  (set `self.Is Falling` (`NavMovementComponent.IsFalling` (`self.CharacterMovement`)))
  (bind _flipbook (`self.AnimationStateMachine` (`self.Is Falling`) (`self.Is Moving`)))
  (`PaperFlipbookComponent.SetFlipbook` (`self.Sprite`) _flipbook))

(fn `AnimationStateMachine`
  (params (IsFalling :type Boolean) (IsMoving :type Boolean))
  (returns (Flipbook :type "PaperFlipbook Object Reference"))
  (locals (AnimationState :type "/Game/Data/AnimationState Enum") (IsFallingLocal :type Boolean) (IsMovingLocal :type Boolean))
  (set `local.IsFallingLocal` IsFalling)
  (set `local.IsMovingLocal` IsMoving)
  (if (`local.IsFallingLocal`)
    (set `local.AnimationState` "NewEnumerator2")
    (elif (`local.IsMovingLocal`)
      (set `local.AnimationState` "NewEnumerator1")
      (else
        (set `local.AnimationState` "NewEnumerator0"))))
  (return (select `/Game/Data/AnimationState` (`local.AnimationState`) :`NewEnumerator0` (`self.IdleFlipbook`) :`NewEnumerator1` (`self.RunFlipbook`) :`NewEnumerator2` (`self.JumpFlipbook`))))

(fn `UserConstructionScript`)