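; Moving spike hazard that kills Player1 or Player2 when they overlap its KillZone.
; LiftTimeline lerps the sprite between its origin and EndLocation at a rate set by TravelTimeInSeconds, reversing after StopDelay to loop.
; BeginPlay only configures it; nothing in this graph makes the first LiftForward call.
; The construction script sets tint and sort priority, and previews the end position through TestEndLocation.
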(event `self.ReceiveBeginPlay`
  (`TimelineComponent.SetPlayRate` (`self.LiftTimeline`) (/ 1.0 (`self.TravelTimeInSeconds`)))
  (set `self.TestEndLocation` true))

(event `self.KillZone.OnComponentBeginOverlap`
  (params (OverlappedComponent :type "PrimitiveComponent Object Reference") (OtherActor :type "Actor Object Reference") (OtherComp :type "PrimitiveComponent Object Reference") (OtherBodyIndex :type Integer) (bFromSweep :type Boolean) (SweepResult :type "HitResult Structure (by ref)"))
  (`|ExecutionSequence`
    (:`then_0`
      (bind _asplayer_2 (cast `/Game/Blueprint/Player2` OtherActor))
      (`/Game/Blueprint/Player2.Death` _asplayer_2))
    (:`then_1`
      (bind _asplayer_1 (cast `/Game/Blueprint/Player1` OtherActor))
      (`/Game/Blueprint/Player1.Death` _asplayer_1))))

(event `LiftForward`
  (bind (_direction _lerp_alpha) (`Timeline|LiftTimeline` :!via `PlayFromStart` :!label _label)
    (:`Update`
      (`SceneComponent.K2_SetRelativeLocation` (`self.SpikesSprite`) (`KismetMathLibrary.VLerp` (0.0 0.0 0.0) (`self.EndLocation`) _lerp_alpha) false false))
    (:`Finished`
      (`KismetSystemLibrary.Delay` (`self.StopDelay`))
      (switch `ETimelineDirection` _direction
        (:`Forward`
          (`self.LiftBack`))
        (:`Backward`
          (`self.LiftForward`))))))

(event `LiftBack`
  (goto _label :!via `ReverseFromEnd`))

(fn `UserConstructionScript`
  (bind _spikessprite (`self.SpikesSprite`))
  (`PrimitiveComponent.SetTranslucentSortPriority` (`self.SpikesSprite`) -1)
  (`SceneComponent.K2_SetRelativeLocation` _spikessprite (`KismetMathLibrary.SelectVector` (`self.EndLocation`) (0.0 0.0 0.0) (`self.TestEndLocation`)) false false)
  (`PaperSpriteComponent.SetSpriteColor` _spikessprite (`self.LiftColor`)))