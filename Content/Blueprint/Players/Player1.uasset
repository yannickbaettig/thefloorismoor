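; Player 1's side-scrolling flipbook character, which moves on X, jumps, and on death disables input and shows the GameOver widget.
; Tick derives jump and fall flags from velocity, feeding a state-selection function that sets the sprite's flipbook.
; A DoOnce gates the attached running sound, stopped when idle or jumping.
; It also receives Player 2's move, jump and crouch input, relaying it to Player2 actors found by class.
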(event `self.ReceiveTick`
  (params (DeltaSeconds :type "Float (single-precision)"))
  (`self.JumpingAnimation`)
  (`self.PlaySound`))

(event `InputAxis|MoveRightPlayer1`
  (params (AxisValue :type "Float (single-precision)"))
  ;[1 1 1] Movement
  (`self.AddMovementInput` (1.0 0.0 0.0) AxisValue)
  (`self.UpdateAnimation`)
  (`/Engine/EditorBlueprintResources/StandardMacros.CompareFloat` AxisValue
    (:`>`
      (`Controller.SetControlRotation` (`self.GetController`) (`KismetMathLibrary.MakeRotator` 0.0)))
    (:`<`
      (`Controller.SetControlRotation` (`self.GetController`) (`KismetMathLibrary.MakeRotator` 0.0 0.0 180.0)))))

(event `InputAction|JumpPlayer1`
  (params (Key :type "Key Structure"))
  ;[1 1 1] Jumping
  (:`Pressed`
    (`self.Jump`)
    (`self.StopSound`))
  (:`Released`
    (`self.StopJumping`)))

(event `UpdateAnimation`
  ;[1 1 1] Animation
  (set `self.Is Moving` (!= (.x (`self.GetVelocity`)) 0.0))
  (bind _flipbook (`self.AnimationStateMachine` (`self.IsDead`) (`self.Is Falling`) (`self.IsJumping`) (`self.Is Moving`) :!label _label))
  (`PaperFlipbookComponent.SetFlipbook` (`self.Sprite`) _flipbook)
  (`PaperFlipbookComponent.SetLooping` (`self.Sprite`) (!= (`self.IsDead`) true)))

(event `JumpingAnimation`
  ;[1 1 1] Animation
  (if (`NavMovementComponent.IsFalling` (`self.CharacterMovement`))
    (if (> (.z (`self.GetVelocity`)) 0.0)
      (set `self.IsJumping` true)
      (goto _label)
      (else
        (set `self.Is Falling` true)
        (goto _label)))
    (else
      (set `self.IsJumping` false)
      (set `self.Is Falling` false)
      (goto _label))))

(event `StopSound`
  (bind _runningsound (`self.RunningSound`))
  (if (`KismetSystemLibrary.IsValid` _runningsound)
    (`AudioComponent.Stop` _runningsound)
    (goto _label_3 :!via `Reset`)))

(event `InputAxis|MoveRightPlayer2`
  (params (AxisValue :type "Float (single-precision)"))
  ;[1 1 1] Movement Player2
  (bind _outactors (`GameplayStatics.GetAllActorsOfClass` "/Game/Blueprint/Players/Player2.Player2_C"))
  (message `/Game/Blueprint/Players/1pTo2pInterface.Call2PMovement` _outactors AxisValue))

(event `InputAction|JumpPlayer2`
  (params (Key :type "Key Structure"))
  ;[1 1 1] Movement Player2
  (:`Pressed`
    (set `self.IsReleasedJump` false)
    (bind _outactors (`GameplayStatics.GetAllActorsOfClass` "/Game/Blueprint/Players/Player2.Player2_C" :!label _label_2))
    (`/Game/Blueprint/Players/1pTo2pInterface.Call2PJumping` _outactors (`self.IsReleasedJump`)))
  (:`Released`
    (set `self.IsReleasedJump` true)
    (goto _label_2)))

(event `PlaySound`
  ;[1 1 1] sound
  (if (or (`self.IsDead`) (`self.IsJumping`))
    _
    (elif (`self.Is Moving`)
      (`/Engine/EditorBlueprintResources/StandardMacros.DoOnce` false :!label _label_3
        (:`Completed`
          (bind _returnvalue (`GameplayStatics.SpawnSoundAttached` "/Game/sound/running_Cue1.running_Cue1" (`self.Sprite`)))
          (set `self.RunningSound` _returnvalue)))
      (else
        (`self.StopSound`)))))

(event `InputAction|CrouchPlayer2`
  (params (Key :type "Key Structure"))
  ;[1 1 1] Movement Player2
  (:`Pressed`
    (set `self.IsReleasedCrouch` false)
    (bind _outactors (`GameplayStatics.GetAllActorsOfClass` "/Game/Blueprint/Players/Player2.Player2_C" :!label _label_4))
    (`/Game/Blueprint/Players/1pTo2pInterface.Call2PCrouching` _outactors (`self.IsReleasedCrouch`)))
  (:`Released`
    (set `self.IsReleasedCrouch` true)
    (goto _label_4)))

(fn `AnimationStateMachine`
  (params (IsDead :type Boolean) (IsFalling :type Boolean) (IsJumping :type Boolean) (IsMoving :type Boolean))
  (returns (Flipbook :type "PaperFlipbook Object Reference"))
  (locals (AnimationState :type "/Game/Data/AnimationState Enum") (IsFallingLocal :type Boolean) (IsMovingLocal :type Boolean))
  (if IsDead
    (set `local.AnimationState` "NewEnumerator3")
    (elif IsFalling
      (set `local.AnimationState` "NewEnumerator4")
      (elif IsJumping
        (set `local.AnimationState` "NewEnumerator2")
        (elif IsMoving
          (set `local.AnimationState` "NewEnumerator1")
          (else
            (set `local.AnimationState` "NewEnumerator0"))))))
  (return (select `/Game/Data/AnimationState` (`local.AnimationState`) :`NewEnumerator0` (`self.IdleFlipbook`) :`NewEnumerator1` (`self.RunFlipbook`) :`NewEnumerator2` (`self.JumpFlipbook`) :`NewEnumerator3` (`self.DeathFlipbook`) :`NewEnumerator4` (`self.FallingFlipbook`))))

(fn `Death`
  (set `self.IsDead` true)
  (`self.UpdateAnimation`)
  (`GameplayStatics.PlaySound2D` "/Game/sound/death_male_Cue.death_male_Cue")
  (`self.DisableInput` null)
  (bind _returnvalue (`|CreateWidget` "/Game/Blueprint/Screens/GameOver.GameOver_C"))
  (`UserWidget.AddToViewport` _returnvalue 0)
  (bind _asplayer_controller (cast `PlayerController` (`GameplayStatics.GetPlayerController` 0)))
  (set `PlayerController.bShowMouseCursor` true _asplayer_controller))

(fn `UserConstructionScript`)