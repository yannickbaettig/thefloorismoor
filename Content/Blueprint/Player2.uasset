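; Paper2D character for the second player, exposing events for horizontal movement with facing flips, jumping and crouching.
; Tick derives jump and fall flags, rescales the sprite for crouching and starts or stops an attached running sound through a DoOnce.
; AnimationStateMachine picks the flipbook by priority from death, falling, jumping and moving flags.
; Death disables player pawn 0's input and shows the GameOver widget with the mouse cursor.
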(event `self.ReceiveBeginPlay`)

(event `self.ReceiveTick`
  (params (DeltaSeconds :type "Float (single-precision)"))
  (`self.JumpingAnimation`)
  (`self.ChecKIfCrouched`)
  (`self.PlaySound`))

(event `/Game/Blueprint/1pTo2pInterface.Call2PMovement`
  (params (Value :type "Float (single-precision)"))
  ;[1 1 1] Movement
  (`self.AddMovementInput` (1.0 0.0 0.0) Value)
  (`self.Update Animation`)
  (`/Engine/EditorBlueprintResources/StandardMacros.CompareFloat` Value
    (:`>`
      (`Controller.SetControlRotation` (`self.GetController`) (`KismetMathLibrary.MakeRotator` 0.0)))
    (:`<`
      (`Controller.SetControlRotation` (`self.GetController`) (`KismetMathLibrary.MakeRotator` 0.0 0.0 180.0)))))

(event `/Game/Blueprint/1pTo2pInterface.Call2PCrouching`
  (params (Released :type Boolean))
  ;[1 1 1] Crouching
  (if Released
    (`self.UnCrouch`)
    (else
      (`self.Crouch`))))

(event `/Game/Blueprint/1pTo2pInterface.Call2PJumping`
  (params (Released :type Boolean))
  ;[1 1 1] Jumping
  (if Released
    (`self.StopJumping`)
    (else
      (`self.Jump`))))

(event `CheckIfCrouched`
  ;[1 1 1] Crouching
  (if (`self.bIsCrouched`)
    (`SceneComponent.SetWorldScale3D` (`self.Sprite`) (`self.CrouchScale`))
    (else
      (`SceneComponent.SetWorldScale3D` (`self.Sprite`) (1.0 1.0 1.0)))))

(event `Update Animation`
  ;[1 1 1] Animation
  (set `self.Is Moving` (!= (.x (`self.GetVelocity`)) 0.0))
  (bind _flipbook (`self.AnimationStateMachine` (`self.IsDead`) (`self.Is Falling`) (`self.IsJumping`) (`self.Is Moving`) :!label _label))
  (`PaperFlipbookComponent.SetFlipbook` (`self.Sprite`) _flipbook)
  (`PaperFlipbookComponent.SetLooping` (`self.Sprite`) (!= (`self.IsDead`) true)))

(event `PlaySound`
  (bind _runningsound (`self.RunningSound`))
  ;[1 1 1] sound
  (if (or (`self.IsDead`) (`self.IsJumping`))
    _
    (elif (`self.Is Moving`)
      (`/Engine/EditorBlueprintResources/StandardMacros.DoOnce` false :!label _label_2
        (:`Completed`
          (bind _returnvalue (`GameplayStatics.SpawnSoundAttached` "/Game/sound/running_Cue.running_Cue" (`self.Sprite`)))
          (set `self.RunningSound` _returnvalue)))
      (elif (`KismetSystemLibrary.IsValid` _runningsound)
        (`AudioComponent.Stop` _runningsound)
        (goto _label_2 :!via `Reset`)))))

(event `JumpingAnimation`
  ;[1 1 1] Animation
  (if (`NavMovementComponent.IsFalling` (`self.CharacterMovement`))
    (if (> (.z (`self.GetVelocity`)) 0.0)
      (set `self.IsJumping` true)
      (goto _label)
      (else
        (set `self.Is Falling` true)
        (goto _label)))
    (else
      (set `self.IsJumping` false)
      (set `self.Is Falling` false)
      (goto _label))))

(fn `AnimationStateMachine`
  (params (IsDead :type Boolean) (IsFalling :type Boolean) (IsJumping :type Boolean) (IsMoving :type Boolean))
  (returns (Flipbook :type "PaperFlipbook Object Reference"))
  (locals (AnimationState :type "/Game/Data/AnimationState Enum"))
  (if IsDead
    (set `local.AnimationState` "NewEnumerator3")
    (elif IsFalling
      (set `local.AnimationState` "NewEnumerator4")
      (elif IsJumping
        (set `local.AnimationState` "NewEnumerator2")
        (elif IsMoving
          (set `local.AnimationState` "NewEnumerator1")
          (else
            (set `local.AnimationState` "NewEnumerator0"))))))
  (return (select `/Game/Data/AnimationState` (`local.AnimationState`) :`NewEnumerator0` (`self.IdleFlipbook`) :`NewEnumerator1` (`self.RunFlipbook`) :`NewEnumerator2` (`self.JumpFlipbook`) :`NewEnumerator3` (`self.DeathFlipbook`) :`NewEnumerator4` (`self.FallingFlipbook`))))

(fn `Death`
  (set `self.IsDead` true)
  (`self.Update Animation`)
  (`self.DisableInput` (`GameplayStatics.GetPlayerPawn` 0) null)
  (bind _returnvalue (`|CreateWidget` "/Game/Blueprint/GameOver.GameOver_C"))
  (`UserWidget.AddToViewport` _returnvalue 0)
  (bind _asplayer_controller (cast `PlayerController` (`GameplayStatics.GetPlayerController` 0)))
  (set `PlayerController.bShowMouseCursor` true _asplayer_controller))

(fn `UserConstructionScript`)