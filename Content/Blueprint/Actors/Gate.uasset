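; Moving gate actor whose sprite slides between its origin and EndLocation, with an overlap KillZone that kills Player1 or Player2.
; A timeline scaled to the travel time drives the motion, starting on BeginPlay unless OpenOnActivate is set.
; Each move plays an attached chain sound that fades out on finish, then after a delay the gate can reverse to loop when Repeat is set.
; The construction script previews the end position through TestEndLocation.
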(event `self.ReceiveBeginPlay`
  (`TimelineComponent.SetPlayRate` (`self.GateTimeline`) (/ 1.0 (`self.TravelTimeInSeconds`)))
  (set `self.TestEndLocation` true)
  (if (not (`self.OpenOnActivate`))
    (`self.GateForward`)))

(event `GateForward`
  (bind _returnvalue (`GameplayStatics.SpawnSoundAttached` "/Game/sound/metal_chain_Cue.metal_chain_Cue" (`self.Sprite`)))
  (set `self.GateSound` _returnvalue)
  (bind (_direction _lerp_alpha) (`Timeline|GateTimeline` :!via `PlayFromStart` :!label _label)
    (:`Update`
      (`SceneComponent.K2_SetRelativeLocation` (`self.Sprite`) (`KismetMathLibrary.VLerp` (0.0 0.0 0.0) (`self.EndLocation`) _lerp_alpha) false false))
    (:`Finished`
      (`AudioComponent.FadeOut` (`self.GateSound`) 0.3 0.0)
      (`KismetSystemLibrary.Delay` (`self.StopDelay`))
      (switch `ETimelineDirection` _direction
        (:`Forward`
          (if (`self.Repeat`)
            (`self.GateBackward`)))
        (:`Backward`
          (`self.GateForward`))))))

(event `self.KillZone.OnComponentBeginOverlap`
  (params (OverlappedComponent :type "PrimitiveComponent Object Reference") (OtherActor :type "Actor Object Reference") (OtherComp :type "PrimitiveComponent Object Reference") (OtherBodyIndex :type Integer) (bFromSweep :type Boolean) (SweepResult :type "HitResult Structure (by ref)"))
  ;[1 1 1] Kill Player
  (`|ExecutionSequence`
    (:`then_0`
      (bind _asplayer_2 (cast `/Game/Blueprint/Players/Player2` OtherActor))
      (`/Game/Blueprint/Players/Player2.Death` _asplayer_2))
    (:`then_1`
      (bind _asplayer_1 (cast `/Game/Blueprint/Players/Player1` OtherActor))
      (`/Game/Blueprint/Players/Player1.Death` _asplayer_1))))

(event `GateBackward`
  (bind _returnvalue (`GameplayStatics.SpawnSoundAttached` "/Game/sound/metal_chain_Cue.metal_chain_Cue" (`self.Sprite`)))
  (set `self.GateSound` _returnvalue)
  (goto _label :!via `ReverseFromEnd`))

(fn `UserConstructionScript`
  (`SceneComponent.K2_SetRelativeLocation` (`self.Sprite`) (`KismetMathLibrary.SelectVector` (`self.EndLocation`) (0.0 0.0 0.0) (`self.TestEndLocation`)) false false))