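; Switchable spikes actor that rotates between zero rotation and DesiredRotation using door-style timeline logic.
; DoorForward plays a sound and lerps the rotation along DoorTimeline, then after StopDelay calls DoorBackward to reverse it if CloseAgain is set.
; Activate only sets the play rate from TravelTimeInSeconds and raises TestEndLocation, with no call to DoorForward here.
; The construction script uses TestEndLocation to preview the start or end rotation.
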(event `Activate`
  (`TimelineComponent.SetPlayRate` (`self.DoorTimeline`) (/ 1.0 (`self.TravelTimeInSeconds`)))
  (set `self.TestEndLocation` true))

(event `DoorForward`
  (`GameplayStatics.PlaySound2D` "/Game/sound/door_Cue.door_Cue")
  (bind (_direction _opendoor) (`Timeline|DoorTimeline` :!label _label)
    (:`Update`
      (`self.K2_SetActorRotation` (`KismetMathLibrary.RLerp` (struct) (`self.DesiredRotation`) _opendoor)))
    (:`Finished`
      (`KismetSystemLibrary.Delay` (`self.StopDelay`))
      (switch `ETimelineDirection` _direction
        (:`Forward`
          (if (`self.CloseAgain`)
            (`self.DoorBackward`)))))))

(event `DoorBackward`
  (`GameplayStatics.PlaySound2D` "/Game/sound/door_Cue.door_Cue")
  (goto _label :!via `ReverseFromEnd`))

(fn `UserConstructionScript`
  (`self.K2_SetActorRotation` (`KismetMathLibrary.SelectRotator` (`self.DesiredRotation`) (struct) (`self.TestEndLocation`))))