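; Baby actor that acts as a goal trigger: either player touching its Capsule loads MainMenuLevel.
; A separate BabySound overlap volume spawns the Baby_Cue sound attached to the root and fades it in slowly when Player1 or Player2 enters.
; When either player leaves that volume, the last spawned sound fades out.
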(event `self.Capsule.OnComponentBeginOverlap`
  (params (OverlappedComponent :type "PrimitiveComponent Object Reference") (OtherActor :type "Actor Object Reference") (OtherComp :type "PrimitiveComponent Object Reference") (OtherBodyIndex :type Integer) (bFromSweep :type Boolean) (SweepResult :type "HitResult Structure (by ref)"))
  (`|ExecutionSequence`
    (:`then_0`
      (cast `/Game/Blueprint/Players/Player2` OtherActor))
    (:`then_1`
      (cast `/Game/Blueprint/Players/Player1` OtherActor)))
  (`GameplayStatics.OpenLevel` "MainMenuLevel"))

(event `self.BabySound.OnComponentBeginOverlap`
  (params (OverlappedComponent :type "PrimitiveComponent Object Reference") (OtherActor :type "Actor Object Reference") (OtherComp :type "PrimitiveComponent Object Reference") (OtherBodyIndex :type Integer) (bFromSweep :type Boolean) (SweepResult :type "HitResult Structure (by ref)"))
  (`|ExecutionSequence`
    (:`then_0`
      (cast `/Game/Blueprint/Players/Player2` OtherActor))
    (:`then_1`
      (cast `/Game/Blueprint/Players/Player1` OtherActor)))
  (bind _returnvalue (`GameplayStatics.SpawnSoundAttached` "/Game/sound/baby_Cue.baby_Cue" (`self.RootComponent`)))
  (`AudioComponent.FadeIn` _returnvalue 10.0 1.0 0.0))

(event `self.BabySound.OnComponentEndOverlap`
  (params (OverlappedComponent :type "PrimitiveComponent Object Reference") (OtherActor :type "Actor Object Reference") (OtherComp :type "PrimitiveComponent Object Reference") (OtherBodyIndex :type Integer))
  (`|ExecutionSequence`
    (:`then_0`
      (cast `/Game/Blueprint/Players/Player2` OtherActor))
    (:`then_1`
      (cast `/Game/Blueprint/Players/Player1` OtherActor)))
  (`AudioComponent.FadeOut` (stale `self.BabySound.OnComponentBeginOverlap` _returnvalue) 5.0 0.0))

(fn `UserConstructionScript`)